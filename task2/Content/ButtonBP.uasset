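; A clickable button Blueprint that spawns a turtle at a linked Nest actor.
; On click, the button mesh briefly dips and returns while a TurtleBP spawns, receives this button's two-stage speed and duration settings, and a spawn sound and particle effect play.
; The construction script applies a configurable material to the button mesh, so placed instances can differ in look and turtle movement.
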(event `self.Button.OnClicked`
  (params (TouchedComponent :type "PrimitiveComponent Object Reference") (ButtonPressed :type "Key Structure"))
  (`|ExecutionSequence`
    (:`then_0`
      ;[1 1 1] Анимация кнопки
      (`SceneComponent.K2_SetRelativeLocation` (`self.Button`) (0.0 0.0 -10.0) false false)
      (`KismetSystemLibrary.Delay` 0.1)
      (`SceneComponent.K2_SetRelativeLocation` (`self.Button`) (0.0 0.0 0.0) false false))
    (:`then_1`
      ;[1 1 1] Создание и настройка черепашки
      (bind _returnvalue (`|SpawnActorFromClass` "/Game/TurtleBP.TurtleBP_C" (`KismetMathLibrary.MakeTransform` (`self.K2_GetActorLocation` (`self.Nest`))) "Undefined" "OverrideRootScale" null null))
      (`self.turtleSpeedUpdate` _returnvalue)
      ;[1 1 1] Активация звука и эффекта появления
      (`GameplayStatics.PlaySoundAtLocation` "/Game/Sounds/sound1.sound1" (`self.K2_GetActorLocation` (`self.Nest`)) (struct) 1.0 1.0 0.0 null null null)
      (`ActorComponent.Activate` (`self.ParticleSystem`) true))))

(fn `turtleSpeedUpdate`
  (params (turtle :type "/Game/TurtleBP Object Reference"))
  ;[1 1 1] Функция передает правила передвижения черепашке
  (set `/Game/TurtleBP.FirstSpeed` (`self.firstSpeed`) turtle)
  (set `/Game/TurtleBP.FirstSpeedDuration` (`self.firstSpeedDuration`) turtle)
  (set `/Game/TurtleBP.SecondSpeed` (`self.secondSpeed`) turtle)
  (set `/Game/TurtleBP.SecondSpeedDuration` (`self.secondSpeedDuration`) turtle))

(fn `UserConstructionScript`
  (`PrimitiveComponent.SetMaterial` (`self.Button`) 1 (`self.Material`)))