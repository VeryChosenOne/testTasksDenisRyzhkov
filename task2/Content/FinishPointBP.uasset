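; FinishPointBP is a finish point actor that destroys any actor that begins overlapping its Box component, with no type check.
; On overlap it also activates its ParticleSystem and plays a sound at its own location.
; The construction script gives the StaticMesh a small random horizontal offset and random yaw at half scale, so placed instances vary visually.
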(event `self.Box.OnComponentBeginOverlap`
  (params (OverlappedComponent :type "PrimitiveComponent Object Reference") (OtherActor :type "Actor Object Reference") (OtherComp :type "PrimitiveComponent Object Reference") (OtherBodyIndex :type Integer) (bFromSweep :type Boolean) (SweepResult :type "HitResult Structure (by ref)"))
  ;[1 1 1] При сталкновении, уничтожает актора, активирует эффект и звук
  (`self.K2_DestroyActor` OtherActor)
  (`ActorComponent.Activate` (`self.ParticleSystem`) true)
  (`GameplayStatics.PlaySoundAtLocation` "/Game/Sounds/sound3.sound3" (`self.K2_GetActorLocation`) (struct) 1.0 1.0 0.0 null null null))

(fn `UserConstructionScript`
  (`SceneComponent.K2_SetRelativeTransform` (`self.StaticMesh`) (`KismetMathLibrary.MakeTransform` (`KismetMathLibrary.MakeVector` (`KismetMathLibrary.RandomFloatInRange` -20.0 20.0) (`KismetMathLibrary.RandomFloatInRange` -20.0 20.0)) (`KismetMathLibrary.MakeRotator` 0.0 0.0 (`KismetMathLibrary.RandomFloatInRange` 0.0 359.0)) (0.5 0.5 0.5)) false false))